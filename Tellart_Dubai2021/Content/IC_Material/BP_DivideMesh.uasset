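; BP_DivideMesh is an early procedural mesh actor that builds a mesh section from its geometry arrays and assigns a material.
; The Construction Script passes the vertex, triangle, normal, UV and tangent arrays to the ProceduralMesh component.
; DrawTriangle sets one triangle's vertices and indices, but its call is disconnected, as is the call to DrawQuad.
; DrawQuad and ClearMeshData are empty stubs, and no mesh-division logic is present.
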(event EventBeginPlay)

(event Collision|EventActorBeginOverlap
  (params (OtherActor :type Actor%20Object%20Reference)))

(event EventTick
  (params (DeltaSeconds :type Float%20%28single-precision%29)))

(fn ConstructionScript
  (bind _proceduralmesh (Variables|Default|GetProceduralMesh))
  (Class|ProceduralMeshComponent|CreateMeshSectionLinearColor _proceduralmesh 0 (Variables|Default|GetVertex) (Variables|Default|GetTriangle) (Variables|Default|GetNormal) (Variables|Default|GetUV) 0 0 0 0 (Variables|Default|GetTangent) false)
  (Rendering|Material|SetMaterial _proceduralmesh 0 (Variables|Default|GetMaterial)))

(fn DrawTriangle
  (Variables|Default|SetVertex (Utilities|Array|MakeArray "0, 0, 0" "0, 0,100.000000" "100.000000, 0, 0"))
  (Variables|Default|SetTriangle (Utilities|Array|MakeArray 2 1 0)))

(fn DrawQuad)

(fn ClearMeshData)